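; MyPlayer is a player Blueprint with basic movement and a test health system.
; Each Tick it builds a world-space offset from the forward and right move inputs, speed and delta time, applies it without sweep, and turns the Cube component to face that direction.
; A Hurt Player input action subtracts a temporary damage value from current health and prints the result, with no clamping or death handling.
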(event `self.ReceiveTick`
  (params (DeltaSeconds :type "Float (single-precision)"))
  (bind _returnvalue (* (`KismetMathLibrary.MakeVector` (`self.GetInputAxisValue`) (`self.GetInputAxisValue`)) (* DeltaSeconds (`self.Movement Speed`))))
  ;[0.1277 0.2754 1] Basic Player Movement and Rotation
  (if (> (`KismetMathLibrary.VSize` _returnvalue) 0.0)
    (`self.K2_AddActorWorldTransform` (`KismetMathLibrary.Conv_VectorToTransform` _returnvalue))
    (`SceneComponent.K2_SetWorldRotation` (`self.Cube`) (`KismetMathLibrary.Conv_VectorToRotator` _returnvalue) false false)))

(event `InputAction|Hurt Player`
  (params (Key :type "Key Structure"))
  ;[1 0.08281 0.07286] Basic Health Calculation
  (:`Pressed`
    (set `self.Current Health` (- (`self.Current Health`) (`self.(TEMP) Damage`)))
    (`KismetSystemLibrary.PrintString` (`KismetStringLibrary.Conv_DoubleToString` (`self.Current Health`)))))

(fn `UserConstructionScript`)