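; Player-fired projectile actor that damages enemies and shoots down enemy projectiles, with a 20-second lifetime.
; On any overlap it calls DestroyActor first, then casts the other actor to four enemy character classes to call EnemyDamage.
; An Enemy_Projectile hit calls GotShot, then destroys again if the player's CanPenatrate flag is off, so the initial destroy overrides penetration.
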(event `self.ReceiveBeginPlay`
  ;[0 1 0.2868] Begin Play
  (`KismetSystemLibrary.Delay` 20.0)
  (`self.K2_DestroyActor`))

(event `self.ReceiveActorBeginOverlap`
  (params (OtherActor :type "Actor Object Reference"))
  ;[1 0 0.09678] On Overlap with Enemy_Character, calls the take damage function, checks from the player if the shots can penatrate, and destroys itself if it can't
  (`self.K2_DestroyActor`)
  (bind _asenemy_character (cast `/Game/Enemies/Harri/Chase_Enemy/Enemy_Character` OtherActor)
    (:`then`
      (`/Game/Enemies/Harri/Chase_Enemy/Enemy_Character.Enemy_Damage` _asenemy_character))
    (:`CastFailed`
      _))
  (bind _asenemy_character_2 (cast `/Game/Enemies/Harri/Shoot_Enemy/Enemy_Character_2` OtherActor)
    (:`then`
      (`/Game/Enemies/Harri/Shoot_Enemy/Enemy_Character_2.Enemy_Damage` _asenemy_character_2))
    (:`CastFailed`
      _))
  (bind _asenemy_character_3 (cast `/Game/Enemies/Harri/Charge_Enemy/Enemy_Character_3` OtherActor)
    (:`then`
      (`/Game/Enemies/Harri/Charge_Enemy/Enemy_Character_3.Enemy_Damage` _asenemy_character_3))
    (:`CastFailed`
      _))
  (bind _asenemy_character_4 (cast `/Game/Enemies/Harri/Move_Then_Shoot_Enemy/Enemy_Character_4` OtherActor)
    (:`then`
      (`/Game/Enemies/Harri/Move_Then_Shoot_Enemy/Enemy_Character_4.Enemy_Damage` _asenemy_character_4))
    (:`CastFailed`
      _))
  (bind _asenemy_projectile (cast `/Game/Enemies/Harri/Shoot_Enemy/Enemy_Projectile` OtherActor))
  (`/Game/Enemies/Harri/Shoot_Enemy/Enemy_Projectile.GotShot` _asenemy_projectile)
  (bind _asthird_person_character (cast `/Game/Blueprints/ThirdPersonCharacter` (`GameplayStatics.GetPlayerCharacter` 0)))
  (if (not (`/Game/Blueprints/ThirdPersonCharacter.canPenatrate` _asthird_person_character))
    (`self.K2_DestroyActor`)))

(fn `UserConstructionScript`)