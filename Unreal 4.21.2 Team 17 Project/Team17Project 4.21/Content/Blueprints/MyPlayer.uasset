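; Player Blueprint that provides basic axis-driven movement, with a Cube component that faces the direction of travel.
; Each Tick builds a horizontal vector from the MoveForward and MoveRight inputs, scaled by MovementSpeed and delta time.
; A non-zero vector offsets the actor in world space without sweeping for collision and snaps only the Cube's rotation to that heading.
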(event `self.ReceiveTick`
  (params (DeltaSeconds :type "Float (single-precision)"))
  (bind _returnvalue (* (`KismetMathLibrary.MakeVector` (`self.GetInputAxisValue`) (`self.GetInputAxisValue`)) (* DeltaSeconds (`self.Movement Speed`))))
  ;[0.1277 0.2754 1] Basic Player Movement
  (if (> (`KismetMathLibrary.VSize` _returnvalue) 0.0)
    (`self.K2_AddActorWorldTransform` (`KismetMathLibrary.Conv_VectorToTransform` _returnvalue))
    (`SceneComponent.K2_SetWorldRotation` (`self.Cube`) (`KismetMathLibrary.Conv_VectorToRotator` _returnvalue) false false)))

(fn `UserConstructionScript`)